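; MainPlayer_BP is the player Blueprint, currently set up to test detection of what lies ahead of the follow camera.
; Every Tick it runs an object line trace for WorldDynamic from the FollowCamera along the controller's forward vector.
; It draws the trace for one frame and prints the hit actor's name as debug output.
; An alternative Visibility channel trace remains in the graph but never executes.
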(event `self.ReceiveTick`
  (params (DeltaSeconds :type "Float (single-precision)"))
  (bind _returnvalue (`SceneComponent.K2_GetComponentLocation` (`self.FollowCamera`)))
  (bind _outhit (`KismetSystemLibrary.LineTraceSingleForObjects` :`Start` _returnvalue :`End` (+ _returnvalue (* (`self.GetActorForwardVector` (`self.GetController`)) 1000.0)) :`ObjectTypes` (`|MakeArray` "ObjectTypeQuery2" :!type "EObjectTypeQuery Enum") :`DrawDebugType` "ForOneFrame"))
  (`KismetSystemLibrary.PrintString` (`KismetSystemLibrary.GetDisplayName` (`.HitActor` (`GameplayStatics.BreakHitResult` _outhit)))))

(fn `UserConstructionScript`)