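; First-person player Blueprint that manages the player's health HUD and hurt feedback.
; On BeginPlay it creates the player HUD widget, stores a reference, pushes the current Health to it and adds it to the viewport.
; Custom events refresh the health display and spawn a separate hurt widget each time the player is hurt.
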(event `self.ReceiveBeginPlay`
  (bind _playerhudref (`self.PlayerHUDRef`))
  ;[1 1 1] Initialize Player HUD
  (bind _returnvalue (`|CreateWidget` "/Game/UI/UMG_PlayerHud.UMG_PlayerHUD_C"))
  (set `self.PlayerHUDRef` _returnvalue)
  (`/Game/UI/UMG_PlayerHud.UpdateHealth` _playerhudref (`self.Health`))
  (`UserWidget.AddToViewport` _playerhudref 0))

(event `self.UpdateHealthWidget`
  ;[1 1 1] Update Health Widget
  (`/Game/UI/UMG_PlayerHud.UpdateHealth` (`self.PlayerHUDRef`) (`self.Health`)))

(event `self.PlayerGotHurt`
  ;[1 1 1] Player Hurt Animation Widget
  (bind _returnvalue (`|CreateWidget` "/Game/UI/UMG_PlayerHurt.UMG_PlayerHurt_C"))
  (`UserWidget.AddToViewport` _returnvalue 0))

(fn `UserConstructionScript`)